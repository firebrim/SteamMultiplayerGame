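; Game instance that manages front-end menus, the loading screen and multiplayer sessions.
; Menu events create widgets, mostly cached; hosting creates an Advanced Sessions session named by the server and opens Lobby as a listen server.
; Joining searches sessions and joins a result without selection UI.
; Session and network failures feed a shared error dialog with readable messages, while travel error handling is left unconnected.
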(event EventShowMainMenu
  (bind _returnvalue (Game|GetPlayerController 0))
  ;[1 0 0] Show Main Menu
  (Variables|Widgets|GetMainMenu
    (:then
      _)
    (:else
      (bind _returnvalue_2 (UserInterface|CreateWidget "/Game/UI/MainMenu.MainMenu_C" _returnvalue))
      (bind _output_get (Variables|Widgets|SetMainMenu _returnvalue_2))))
  (UserInterface|Viewport|AddtoViewport _output_get 0)
  (Variables|/Script/Engine.PlayerController|SetbShowMouseCursor _returnvalue true))

(event EventShowHostMenu
  ;[0.6875 1 0] Show Host Menu
  (Variables|Widgets|GetHostMenu
    (:then
      _)
    (:else
      (bind _returnvalue (UserInterface|CreateWidget "/Game/UI/HostMenu.HostMenu_C" (Game|GetPlayerController 0)))
      (bind _output_get (Variables|Widgets|SetHostMenu _returnvalue))))
  (UserInterface|Viewport|AddtoViewport _output_get 0))

(event EventShowServerMenu
  ;[0.7578 0 1] Show Server Menu
  (bind _returnvalue (UserInterface|CreateWidget "/Game/UI/ServerMenu.ServerMenu_C" (Game|GetPlayerController 0)))
  (UserInterface|Viewport|AddtoViewport _returnvalue 0))

(event EventShowOptionsMenu
  ;[1 0.3516 0] Show Options Menu
  (Variables|Widgets|GetOptionsMenu
    (:then
      _)
    (:else
      (bind _returnvalue (UserInterface|CreateWidget "/Game/UI/OptionsMenu.OptionsMenu_C" (Game|GetPlayerController 0)))
      (bind _output_get (Variables|Widgets|SetOptionsMenu _returnvalue))))
  (UserInterface|Viewport|AddtoViewport _output_get 0))

(event EventShowLoadingScreen
  ;[0.2422 0 1] Show Loading Screen
  (Variables|Widgets|GetLoadingScreen
    (:then
      _)
    (:else
      (bind _returnvalue (UserInterface|CreateWidget "/Game/UI/LoadingScreen.LoadingScreen_C" (Game|GetPlayerController 0)))
      (bind _output_get (Variables|Widgets|SetLoadingScreen _returnvalue))))
  (UserInterface|Viewport|AddtoViewport _output_get 0))

(event EventLaunchLobby
  (params (NumberOfPlayers :type Integer) (IsLocalLAN :type Boolean) (ServerName :type Text))
  ;[0.1484 0 1] Launch Lobby
  (Variables|Default|SetNumberOfPlayers NumberOfPlayers)
  (Variables|Default|SetIsLocalLAN IsLocalLAN)
  (Variables|Default|SetServerName ServerName)
  (CallFunction|ShowLoadingScreen)
  (|AdvancedSession (Utilities|Array|MakeArray (Class|AdvancedSessionsLibrary|MakeLiteralSessionPropertyString "servername" (Utilities|String|ToString(Text) (Variables|Default|GetServerName)))) (Game|GetPlayerController 0) (Variables|Default|GetNumberOfPlayers) 0 (Variables|Default|GetIsLocalLAN) true false true true false false false true
    (:OnSuccess
      (Game|OpenLevel(byName) "Lobby" true "listen"))
    (:OnFailure
      (Utilities|ShowErrorDialog "Session error" "Failed to create a new session. Please try again."))))

(event EventJoinServer
  (params (SessionToJoin :type Blueprint%20Session%20Result%20Structure))
  ;[1 0 0.1875] Join Server
  (CallFunction|ShowLoadingScreen)
  (bind _results (|FindSessionsAdvanced (Game|GetPlayerController 0) 20 (Variables|Default|GetIsLocalLAN) "AllServers" 0 false false false 1)
    (:OnSuccess
      (for _array_element _results
        _)
      (|JoinSession (Game|GetPlayerController 0) _array_element
        (:OnFailure
          (Utilities|ShowErrorDialog "Session error" "Failed to join server. Please try again later."))))))

(event EventHandleNetworkError
  (params (FailureType :type ENetworkFailure%20Enum :default "NetDriverAlreadyExists") (bIsServer :type Boolean))
  ;[0.6406 0 1] Network Error Handling
  (if bIsServer
    _
    (else
      _))
  (Utilities|ShowErrorDialog "Network error" (CallFunction|NetworkErrortoString FailureType)))

(event EventHandleTravelError
  (params (FailureType :type ETravelFailure%20Enum :default "NoLevel"))
  ;[0.6406 0 1] Network Error Handling
)

(event EventDestroySessionCaller
  (params (PlayerController :type Player%20Controller%20Object%20Reference))
  ;[0.3359 1 0] Destroy Session
  (|DestroySession PlayerController))

(fn NetworkErrortoString
  (params (Error :type ENetworkFailure%20Enum :default "NetDriverAlreadyExists"))
  (switch Utilities|FlowControl|Switch|SwitchonENetworkFailure Error
    (:NetDriverAlreadyExists
      (LocalVariables|SetErrorString "Network connection lost." :!label _label))
    (:NetDriverCreateFailure
      (goto _label))
    (:NetDriverListenFailure
      (goto _label))
    (:ConnectionLost
      (goto _label))
    (:ConnectionTimeout
      (LocalVariables|SetErrorString "Network connection timeout."))
    (:FailureReceived
      (goto _label))
    (:OutdatedClient
      (goto _label))
    (:OutdatedServer
      (goto _label))
    (:PendingConnectionFailure
      (goto _label))
    (:NetGuidMismatch
      (goto _label))
    (:NetChecksumMismatch
      (goto _label)))
  (return (LocalVariables|GetErrorString)))

(fn TravelErrortoString
  (params (Error :type ETravelFailure%20Enum :default "NoLevel"))
  (switch Utilities|FlowControl|Switch|SwitchonETravelFailure Error
    (:NoLevel
      (LocalVariables|SetErrorString "No Level found."))
    (:LoadMapFailure
      (LocalVariables|SetErrorString "Failure while loading level."))
    (:InvalidURL
      (LocalVariables|SetErrorString "Invalid level destination.")))
  (return (LocalVariables|GetErrorString)))

(fn SMPGameInstanceRef
  (return self))